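; Player controller that drives a BP_MyPown pawn along the world Y axis and quits the game on Escape.
; It sets game-only input at BeginPlay and caches the pawn when possessing it.
; The Moving axis applies a swept world offset to that pawn, scaled by Speed and delta time for frame-rate-independent motion.
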(event EventBeginPlay
  (Input|SetInputModeGameOnly self))

(event EventTick
  (params (DeltaSeconds :type Float%20%28single-precision%29)))

(event EventPossess
  (params (PossessedPawn :type Pawn%20Object%20Reference))
  (bind _asbp_my_pown (Utilities|Casting|CastToBP_MyPown PossessedPawn))
  (Variables|Default|SetMyPown _asbp_my_pown))

(event Input|AxisEvents|InputAxisMoving
  (params (AxisValue :type Float%20%28single-precision%29))
  (Transformation|AddActorWorldOffset (Variables|Default|GetMyPown) (Math|Vector|MakeVector 0.0 (* AxisValue (Utilities|Time|GetWorldDeltaSeconds) (Variables|Default|GetSpeed)) 0.0) true))

(event Input|KeyboardEvents|Escape
  (params (Key :type Key%20Structure))
  (:Pressed
    (Game|QuitGame 0 "Quit" false)))

(fn ConstructionScript)