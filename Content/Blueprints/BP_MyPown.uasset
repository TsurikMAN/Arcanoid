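; Player pawn for what appears to be a Breakout-style game, launching BP_Ball actors and tracking lives.
; Positive PullTheBall input spawns a ball at the capsule when neither tracked ball is valid, spending HP and resetting SpeedChange.
; BP_Bonus overlaps on the Cube dispatch by type to events for an extra ball, life or speed changes.
; Tick shows HP in a text render, and ball hits play a sound.
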(event OnComponentBeginOverlap(Cube)
  (params (OverlappedComponent :type Primitive%20Component%20Object%20Reference) (OtherActor :type Actor%20Object%20Reference) (OtherComp :type Primitive%20Component%20Object%20Reference) (OtherBodyIndex :type Integer) (bFromSweep :type Boolean) (SweepResult :type Hit%20Result%20Structure%20%28by%20ref%29))
  (bind _asbp_bonus (Utilities|Casting|CastToBP_Bonus OtherActor))
  (switch Utilities|FlowControl|Switch|SwitchonE_BonusType (Variables|/Game/Blueprints/Bonuses/BP_Bonus.BP_Bonus_C|GetBonus%20Type _asbp_bonus)
    (:NewEnumerator0
      (CallFunction|Event+1Ball))
    (:NewEnumerator1
      (CallFunction|Event+1HP))
    (:NewEnumerator2
      (CallFunction|Event-1HP))
    (:NewEnumerator3
      (CallFunction|Event+Speed))
    (:NewEnumerator4
      (CallFunction|Event-Speed))))

(event Custom|Event%20+Speed
  (Variables|Default|SetSpeed%20Change (* (Variables|Default|GetSpeed%20Change) 1.25)))

(event Custom|Event%20+1Ball
  (bind _returnvalue (CallFunction|SpawnBall))
  (Variables|Default|SetRespawn2 _returnvalue))

(event Custom|Event%20-1HP
  (Variables|Default|SetHP (- (Variables|Default|GetHP) 1)))

(event Custom|Event%20+1HP
  (Variables|Default|SetHP (+ (Variables|Default|GetHP) 1)))

(event Custom|Spawn%20Ball
  (Variables|Default|GetRespawn
    (:then)
    (:else
      (Variables|Default|GetRespawn2
        (:then)
        (:else
          (if (> (Variables|Default|GetHP) 0)
            (bind _returnvalue (CallFunction|SpawnBall))
            (Variables|Default|SetRespawn _returnvalue)
            (Variables|Default|SetHP (- (Variables|Default|GetHP) 1))
            (Variables|Default|SetSpeed%20Change 7e+02)))))))

(event Custom|Event%20-Speed
  (Variables|Default|SetSpeed%20Change (/ (Variables|Default|GetSpeed%20Change) 1.25)))

(event Collision|EventHit
  (params (MyComp :type Primitive%20Component%20Object%20Reference) (Other :type Actor%20Object%20Reference) (OtherComp :type Primitive%20Component%20Object%20Reference) (bSelfMoved :type Boolean) (HitLocation :type Vector :default "0, 0, 0") (HitNormal :type Vector :default "0, 0, 0") (NormalImpulse :type Vector :default "0, 0, 0") (Hit :type Hit%20Result%20Structure%20%28by%20ref%29))
  (Utilities|Casting|CastToBP_Ball Other)
  (Audio|PlaySound2D 0 1.0 1.0 0.0 0 0))

(event EventTick
  (params (DeltaSeconds :type Float%20%28single-precision%29))
  (Rendering|Components|TextRender|SetText (Variables|Default|GetTextRender1) (Utilities|Text|ToText(Integer) (Variables|Default|GetHP))))

(event Input|AxisEvents|InputAxisPullTheBall
  (params (AxisValue :type Float%20%28single-precision%29))
  (if (> AxisValue 0.0)
    (CallFunction|SpawnBall)))

(fn ConstructionScript)

(fn SpawnBall
  (bind _returnvalue (Game|SpawnActorfromClass "/Game/Blueprints/Game_Objects/BP_Ball.BP_Ball_C" (Math|Transform|MakeTransform (Transformation|GetWorldLocation (Variables|Default|GetCapsule))) "AlwaysSpawn" 0 0))
  (return _returnvalue))