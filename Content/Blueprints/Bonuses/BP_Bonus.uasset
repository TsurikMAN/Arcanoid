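; BP_Bonus is a moving bonus pickup that gets a random type and disappears when the BP_MyPown actor touches it.
; The construction script picks one of five BonusType enum values at random and shows its name on a TextRender component.
; Tick moves the actor along a vector scaled by Speed and delta time, without sweeping.
; Overlap with BP_MyPown only destroys the bonus, applying no effect here.
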(event EventBeginPlay)

(event EventTick
  (params (DeltaSeconds :type Float%20%28single-precision%29))
  (Transformation|AddActorWorldOffset (* (* (Variables|Default|GetVector) (Variables|Default|GetSpeed)) DeltaSeconds)))

(event Collision|EventActorBeginOverlap
  (params (OtherActor :type Actor%20Object%20Reference))
  (Utilities|Casting|CastToBP_MyPown OtherActor)
  (Actor|DestroyActor))

(fn ConstructionScript
  (Variables|Default|SetBonus%20Type (Utilities|Select :Index (Math|Random|RandomIntegerinRange 0 4) :Option%200 "NewEnumerator0" :Option%201 "NewEnumerator1" :Option%202 "NewEnumerator2" :Option%203 "NewEnumerator3" :Option%204 "NewEnumerator4"))
  (Rendering|Components|TextRender|SetText (Variables|Default|GetTextRender) (Utilities|Text|ToText(String) (Utilities|String|EnumtoString (Variables|Default|GetBonus%20Type)))))