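; BP_Ball is a ball actor that moves continuously and bounces off whatever blocks it.
; Each Tick it sweeps its Sphere along Direction, scaled by delta time and the SpeedChange value read from the first BP_MyPown found in the world.
; On a blocking hit it reflects Direction about the surface normal and zeroes Z to keep travel horizontal.
; Its own Speed variable is unused.
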(event EventTick
  (params (DeltaSeconds :type Float%20%28single-precision%29))
  (bind _outactors (Actor|GetAllActorsOfClass "/Game/Blueprints/BP_MyPown.BP_MyPown_C"))
  (bind _asbp_my_pown (Utilities|Casting|CastToBP_MyPown (Utilities|Array|Get(acopy) _outactors)))
  (bind _sweephitresult (Transformation|AddWorldOffset (Variables|Default|GetSphere) (* (* (Variables|Default|GetDirection) (Variables|/Game/Blueprints/BP_MyPown.BP_MyPown_C|GetSpeed%20Change _asbp_my_pown)) DeltaSeconds) true false))
  (if (.bBlockingHit (Collision|BreakHitResult _sweephitresult))
    (Variables|Default|SetDirection (Math|Vector|MakeVector (.x (Math|Vector|GetReflectionVector (Variables|Default|GetDirection) (.Normal (Collision|BreakHitResult _sweephitresult)))) (.y (Math|Vector|GetReflectionVector (Variables|Default|GetDirection) (.Normal (Collision|BreakHitResult _sweephitresult)))) 0.0))))

(fn ConstructionScript)