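; BP_Box is a breakable box that loses one BoxHP each time a BP_Ball hits it, playing an explosion sound.
; While HP remains, the hit swaps the cube's material to steel.
; At zero HP it rolls a random integer up to Bonuses, spawns a half-scale BP_Bonus on a zero, then destroys the Cube1 component rather than the actor.
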(event Collision|EventHit
  (params (MyComp :type Primitive%20Component%20Object%20Reference) (Other :type Actor%20Object%20Reference) (OtherComp :type Primitive%20Component%20Object%20Reference) (bSelfMoved :type Boolean) (HitLocation :type Vector :default "0, 0, 0") (HitNormal :type Vector :default "0, 0, 0") (NormalImpulse :type Vector :default "0, 0, 0") (Hit :type Hit%20Result%20Structure%20%28by%20ref%29))
  (Utilities|Casting|CastToBP_Ball Other)
  (Audio|PlaySound2D "/Game/StarterContent/Audio/Explosion01.Explosion01" 0.5 1.0 0.0 0 0)
  (bind _result (Math|Integer|DecrementInt (Variables|Default|GetBox%20HP))
    (:%20%20
      (if (<= _result 0)
        (Variables|Default|SetBonuses (Math|Random|RandomIntegerinRange 0 (Variables|Default|GetBonuses)))
        (if (== (Variables|Default|GetBonuses) 0)
          (Game|SpawnActorfromClass "/Game/Blueprints/Bonuses/BP_Bonus.BP_Bonus_C" (Math|Transform|MakeTransform (Transformation|GetWorldLocation (Variables|Default|GetCube1)) "0, 0, 0" "0.500000,0.500000,0.500000") "AlwaysSpawn" 0 0))
        (Components|DestroyComponent (Variables|Default|GetCube1))
        (else
          (Rendering|Material|SetMaterial (Variables|Default|GetCube1) 0 "/Game/StarterContent/Materials/M_Metal_Steel.M_Metal_Steel"))))))

(fn ConstructionScript)