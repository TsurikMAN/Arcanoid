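; BP_Box_Script is a grid spawner that previews a layout of cubes in the editor and replaces it with BP_Box actors at play.
; The construction script adds static mesh components on an X by Y grid spaced by Padding.
; BeginPlay destroys those previews and spawns boxes from the actor's location at half-Padding world spacing, ignoring its rotation.
; GetCubesForWin returns the length of CubesForWin, which this file never fills.
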(event EventBeginPlay
  (bind _returnvalue (Transformation|GetActorLocation))
  (for _array_element (Variables|Default|GetCubes)
    (Components|DestroyComponent _array_element))
  (for _index (range 0 (Variables|Default|GetX))
    (for _index_2 (range 0 (Variables|Default|GetY))
      (Game|SpawnActorfromClass "/Game/Blueprints/Game_Objects/BP_Box.BP_Box_C" (Math|Transform|MakeTransform (Math|Vector|MakeVector (+ (Math|Conversions|ToFloat(Integer) (* _index (/ (Variables|Default|GetPadding) 2))) (.x _returnvalue)) (+ (Math|Conversions|ToFloat(Integer) (* _index_2 (/ (Variables|Default|GetPadding) 2))) (.y _returnvalue)) (.z _returnvalue))) "AlwaysSpawn" 0 0))))

(fn ConstructionScript
  (for _index (range 0 (Variables|Default|GetX))
    (for _index_2 (range 0 (Variables|Default|GetY))
      (bind _returnvalue (AddComponent|AddStaticMeshComponent false (Math|Transform|MakeTransform (Math|Vector|MakeVector (Math|Conversions|ToFloat(Integer) (* _index (Variables|Default|GetPadding))) (Math|Conversions|ToFloat(Integer) (* _index_2 (Variables|Default|GetPadding))) 0.0))))
      (Utilities|Array|Add (Variables|Default|GetCubes) _returnvalue))))

(fn GetCubesforWin
  (return (Utilities|Array|Length (Variables|Default|GetCubesForWin))))